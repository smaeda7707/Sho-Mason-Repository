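; BP_PickupItem_Child is a pickup item variant that goes into the character's SecondaryItem slot.
; Pickup attaches it to that component, resets the component to the stored original equipped transform, then applies the item's in-hand position offset and rotation.
; Every tick it runs InteractCheck and infers holding from ItemModel's attach parent, disabling collision and gravity while held and restoring them otherwise.
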(event EventBeginPlay
  (|CallParentFunction) ; This node is disabled and will not be called.\nDrag off pins to build functionality.
)

(event Collision|EventActorBeginOverlap
  (params (OtherActor :type Actor%20Object%20Reference))
  (|CallParentFunction OtherActor) ; This node is disabled and will not be called.\nDrag off pins to build functionality.
)

(event EventPickup
  (bind _characterref (Variables|Default|GetCharacterRef))
  (bind _secondaryitem (Variables|/Game/FirstPerson/Blueprints/BP_FirstPersonCharacter.BP_FirstPersonCharacter_C|GetSecondaryItem _characterref))
  (Transformation|AttachComponentToComponent _secondaryitem "" "SnapToTarget" "SnapToTarget" "KeepRelative" true)
  (Transformation|SetRelativeTransform _secondaryitem (Variables|/Game/FirstPerson/Blueprints/BP_FirstPersonCharacter.BP_FirstPersonCharacter_C|GetEquippedItemOrigianlLocation (Variables|Default|GetCharacterRef)) false false)
  (Transformation|SetRelativeTransform _secondaryitem (Math|Conversions|ToTransform(Vector) (+ (Variables|Default|GetPositionOffsetInHand) (.location (Transformation|GetRelativeTransform _secondaryitem)))) false false)
  (Transformation|SetRelativeRotation _secondaryitem (Variables|Default|GetRotationInHand) false false))

(event EventTick
  (params (DeltaSeconds :type Float%20%28single-precision%29))
  (bind _itemmodel (Variables|Default|GetItemModel))
  (CallFunction|InteractCheck)
  (bind _output_get (Variables|Default|SetIsHolding? (== (Variables|/Game/FirstPerson/Blueprints/BP_FirstPersonCharacter.BP_FirstPersonCharacter_C|GetSecondaryItem (Variables|Default|GetCharacterRef)) (Transformation|GetAttachParent _itemmodel))))
  (if _output_get
    (Collision|SetCollisionEnabled _itemmodel "NoCollision")
    (Physics|SetEnableGravity _itemmodel false)
    (else
      (Collision|SetCollisionEnabled _itemmodel "QueryAndPhysics")
      (Physics|SetEnableGravity _itemmodel true))))

(fn ConstructionScript
  (|CallParentFunction))