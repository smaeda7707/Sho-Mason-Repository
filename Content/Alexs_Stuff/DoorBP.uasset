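; DoorBP is an interactable door that swings open or closed when the first-person player interacts with it.
; Tick polls the cached character's IsInteracting flag and HitActor, then opens or closes based on IsOpen.
; One timeline lerps the door mesh's yaw, playing or reversing at rates derived from open and close times, and toggles IsOpen when finished.
; The Interact and UniversalInteract functions are unimplemented stubs.
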(event Custom|Open%20Door
  (bind _door_track (Timeline|Open%20Door%20Time Play)
    (:Update
      (Transformation|SetRelativeRotation (Variables|Default|GetDoor%20SM) (Math|Rotator|MakeRotator 0.0 0.0 (Math|Float|Lerp (Variables|Default|GetClosed%20Door%20Pos) (Variables|Default|GetOpen%20Door%20Pos) _door_track)) false false))
    (:Finished
      (Variables|Default|SetIsOpen? (not (Variables|Default|GetIsOpen?))))))

(event Custom|Close%20Door
  (bind _door_track (Timeline|Open%20Door%20Time Reverse)
    (:Update
      (Transformation|SetRelativeRotation (Variables|Default|GetDoor%20SM) (Math|Rotator|MakeRotator 0.0 0.0 (Math|Float|Lerp (Variables|Default|GetClosed%20Door%20Pos) (Variables|Default|GetOpen%20Door%20Pos) _door_track)) false false))
    (:Finished
      (Variables|Default|SetIsOpen? (not (Variables|Default|GetIsOpen?))))))

(event EventBeginPlay
  (bind _asbp_first_person_character (Utilities|Casting|CastToBP_FirstPersonCharacter (Game|GetPlayerCharacter 0)))
  (Variables|Default|SetCharacterRef _asbp_first_person_character))

(event EventTick
  (params (DeltaSeconds :type Float%20%28single-precision%29))
  (bind _open_door_time (Variables|Default|GetOpen%20Door%20Time))
  (bind _characterref (Variables|Default|GetCharacterRef))
  (if (and (Variables|/Game/FirstPerson/Blueprints/BP_FirstPersonCharacter.BP_FirstPersonCharacter_C|GetIsInteracting? _characterref) (== (Variables|/Game/FirstPerson/Blueprints/BP_FirstPersonCharacter.BP_FirstPersonCharacter_C|GetHit%20Actor _characterref) self))
    (if (not (Variables|Default|GetIsOpen?))
      (Components|Timeline|SetPlayRate _open_door_time (/ 1.0 (Variables|Default|GetOpenTime)))
      (CallFunction|OpenDoor)
      (else
        (Components|Timeline|SetPlayRate _open_door_time (/ 1.0 (Variables|Default|GetCloseTime)))
        (CallFunction|CloseDoor)))))

(fn ConstructionScript)

(fn Interact
  (params (Interactor :type Character%20Object%20Reference)))

(fn UniversalInteract
  (params (Interactor :type Character%20Object%20Reference))
  (return false))