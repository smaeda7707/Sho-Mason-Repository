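; Interactable hinged door Blueprint that toggles between open and closed yaw angles.
; Interact plays or reverses one timeline at a rate set by the open or close time, lerping the door mesh's yaw.
; IsOpen flips only when the timeline finishes.
; A box overlap shows or hides a prompt widget created at BeginPlay; its check compares against the player controller, not the pawn, so it filters no pawns.
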(event OnComponentBeginOverlap(Box)
  (params (OverlappedComponent :type Primitive%20Component%20Object%20Reference) (OtherActor :type Actor%20Object%20Reference) (OtherComp :type Primitive%20Component%20Object%20Reference) (OtherBodyIndex :type Integer) (bFromSweep :type Boolean) (SweepResult :type Hit%20Result%20Structure%20%28by%20ref%29))
  (if (not (== OtherActor (Game|GetPlayerController 0)))
    (UserInterface|Viewport|AddtoViewport (Variables|Default|GetInteract%20Prompt) 0)))

(event OnComponentEndOverlap(Box)
  (params (OverlappedComponent :type Primitive%20Component%20Object%20Reference) (OtherActor :type Actor%20Object%20Reference) (OtherComp :type Primitive%20Component%20Object%20Reference) (OtherBodyIndex :type Integer))
  (if (not (== (Game|GetPlayerController 0) OtherActor))
    (Widget|RemovefromParent (Variables|Default|GetInteract%20Prompt))))

(event Custom|Open%20Door
  (bind _door_track (Timeline|Open%20Door%20Time Play)
    (:Update
      (Transformation|SetRelativeRotation (Variables|Default|GetDoor%20SM) (Math|Rotator|MakeRotator 0.0 0.0 (Math|Float|Lerp (Variables|Default|GetClosed%20Door%20Pos) (Variables|Default|GetOpen%20Door%20Pos) _door_track)) false false))
    (:Finished
      (Variables|Default|SetIsOpen? (not (Variables|Default|GetIsOpen?))))))

(event Custom|Close%20Door
  (bind _door_track (Timeline|Open%20Door%20Time Reverse)
    (:Update
      (Transformation|SetRelativeRotation (Variables|Default|GetDoor%20SM) (Math|Rotator|MakeRotator 0.0 0.0 (Math|Float|Lerp (Variables|Default|GetClosed%20Door%20Pos) (Variables|Default|GetOpen%20Door%20Pos) _door_track)) false false))
    (:Finished
      (Variables|Default|SetIsOpen? (not (Variables|Default|GetIsOpen?))))))

(event EventBeginPlay
  (bind _returnvalue (UserInterface|CreateWidget "/Game/UI/InteractMessage.InteractMessage_C"))
  (Variables|Default|SetInteract%20Prompt _returnvalue))

(fn ConstructionScript)

(fn Interact
  (params (Interactor :type Character%20Object%20Reference))
  (bind _open_door_time (Variables|Default|GetOpen%20Door%20Time))
  (if (not (Variables|Default|GetIsOpen?))
    (Components|Timeline|SetPlayRate _open_door_time (/ 1.0 (Variables|Default|GetOpenTime)))
    (CallFunction|OpenDoor)
    (else
      (Components|Timeline|SetPlayRate _open_door_time (/ 1.0 (Variables|Default|GetCloseTime)))
      (CallFunction|CloseDoor)))
  (return true))