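; BP_Toilet is a task actor for a toilet that the player cleans with a plunger.
; Each Tick polls the first-person character for an interaction hit on this toilet, then finds the BP_Plunger and checks that it is held.
; CleanToilet then stops the checks and marks the task done, with a print string standing in for the animation.
; UniversalInteract is unused and returns false.
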(event Custom|CleanToilet
  (Variables|Default|SetEndTick false)
  (Variables|Default|SetIsTask? false)
  (Development|PrintString "anim")
  (Variables|Default|SetIsDone? true))

(event EventBeginPlay
  (Variables|Default|SetIsTask? true)
  (Variables|Default|SetEndTick true)
  (Variables|Default|SetIsDone? false)
  (bind _asbp_first_person_character (Utilities|Casting|CastToBP_FirstPersonCharacter (Game|GetPlayerCharacter 0)))
  (Variables|Default|SetCharacterRef _asbp_first_person_character))

(event EventTick
  (params (DeltaSeconds :type Float%20%28single-precision%29))
  (bind _characterref (Variables|Default|GetCharacterRef))
  (if (Variables|Default|GetEndTick)
    (if (Variables|Default|GetIsTask?)
      (if (and (Variables|/Game/FirstPerson/Blueprints/BP_FirstPersonCharacter.BP_FirstPersonCharacter_C|GetIsInteracting? _characterref) (== (Variables|/Game/FirstPerson/Blueprints/BP_FirstPersonCharacter.BP_FirstPersonCharacter_C|GetHit%20Actor _characterref) self))
        (bind _returnvalue (Actor|GetActorOfClass "/Game/Tasks/CleanToiletTask/Code/BP_Plunger.BP_Plunger_C"))
        (if (Variables|/Game/Tasks/BP_PickupItem.BP_PickupItem_C|GetIsHolding? _returnvalue)
          (CallFunction|CleanToilet))))))

(fn ConstructionScript)

(fn UniversalInteract
  (params (Interactor :type Character%20Object%20Reference))
  (return false))