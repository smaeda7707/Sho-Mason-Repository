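; Day cycle Blueprint that gates the advance of in-game time behind the player's completion of daily tasks.
; Each Tick looks up the task actors and counts five completed tasks: bed (blanket and pillow), food, shower, pills and all five plates.
; Time of day is capped at the initial time plus an equal fraction of that initial time per completed task, so the clock holds until more tasks are done.
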(event EventBeginPlay)

(event EventTick
  (params (DeltaSeconds :type Float%20%28single-precision%29))
  (bind _returnvalue (Class|DaySequenceActor|GetDayLength))
  (bind _returnvalue_2 (Class|DaySequenceActor|GetInitialTimeOfDay))
  (bind _returnvalue_3 (/ _returnvalue _returnvalue_2))
  (bind _returnvalue_4 (/ _returnvalue _returnvalue_3))
  (Variables|Default|SetNumTasksCompleted 0)
  (bind _returnvalue_5 (Actor|GetActorOfClass "/Game/Tasks/BedTask/Code/BlanketReplace.BlanketReplace_C"))
  (bind _returnvalue_6 (Actor|GetActorOfClass "/Game/Tasks/BedTask/Code/PillowReplace.PillowReplace_C"))
  (bind _returnvalue_7 (Actor|GetActorOfClass "/Game/Tasks/FoodTask/Code/FoodTask.FoodTask_C"))
  (bind _returnvalue_8 (Actor|GetActorOfClass "/Game/Tasks/ShowerTask/Code/ShowerTask.ShowerTask_C"))
  (bind _returnvalue_9 (Actor|GetActorOfClass "/Game/Tasks/PillsTask/Code/PillsPickup.PillsPickup_C"))
  (bind _returnvalue_10 (Actor|GetActorOfClass "/Game/Tasks/DishTask/Code/PlateReplace1.PlateReplace1_C"))
  (bind _returnvalue_11 (Actor|GetActorOfClass "/Game/Tasks/DishTask/Code/PlateReplace2.PlateReplace2_C"))
  (bind _returnvalue_12 (Actor|GetActorOfClass "/Game/Tasks/DishTask/Code/PlateReplace3.PlateReplace3_C"))
  (bind _returnvalue_13 (Actor|GetActorOfClass "/Game/Tasks/DishTask/Code/PlateReplace4.PlateReplace4_C"))
  (bind _returnvalue_14 (Actor|GetActorOfClass "/Game/Tasks/DishTask/Code/PlateReplace5.PlateReplace5_C"))
  (for _array_element (Utilities|Array|MakeArray (and (Variables|/Game/Tasks/BedTask/Code/BlanketReplace.BlanketReplace_C|GetIsDone? _returnvalue_5) (Variables|/Game/Tasks/BedTask/Code/PillowReplace.PillowReplace_C|GetIsDone? _returnvalue_6)) (Variables|/Game/Tasks/FoodTask/Code/FoodTask.FoodTask_C|GetIsDone? _returnvalue_7) (Variables|/Game/Tasks/ShowerTask/Code/ShowerTask.ShowerTask_C|GetIsDone? _returnvalue_8) (Variables|/Game/Tasks/PillsTask/Code/PillsPickup.PillsPickup_C|GetIsDone? _returnvalue_9) (Math|Boolean|ANDBoolean (Variables|/Game/Tasks/DishTask/Code/PlateReplace1.PlateReplace1_C|GetIsDone? _returnvalue_10) (Variables|/Game/Tasks/DishTask/Code/PlateReplace2.PlateReplace2_C|GetIsDone? _returnvalue_11) (Variables|/Game/Tasks/DishTask/Code/PlateReplace3.PlateReplace3_C|GetIsDone? _returnvalue_12) (Variables|/Game/Tasks/DishTask/Code/PlateReplace4.PlateReplace4_C|GetIsDone? _returnvalue_13) (Variables|/Game/Tasks/DishTask/Code/PlateReplace5.PlateReplace5_C|GetIsDone? _returnvalue_14)))
    (if _array_element
      (Variables|Default|SetNumTasksCompleted (+ (Variables|Default|GetNumTasksCompleted) 1))))
  (if (not (< (Class|DaySequenceActor|GetTimeOfDay) (+ (* (/ _returnvalue_4 (Utilities|Array|Length (Utilities|Array|MakeArray (and (Variables|/Game/Tasks/BedTask/Code/BlanketReplace.BlanketReplace_C|GetIsDone? _returnvalue_5) (Variables|/Game/Tasks/BedTask/Code/PillowReplace.PillowReplace_C|GetIsDone? _returnvalue_6)) (Variables|/Game/Tasks/FoodTask/Code/FoodTask.FoodTask_C|GetIsDone? _returnvalue_7) (Variables|/Game/Tasks/ShowerTask/Code/ShowerTask.ShowerTask_C|GetIsDone? _returnvalue_8) (Variables|/Game/Tasks/PillsTask/Code/PillsPickup.PillsPickup_C|GetIsDone? _returnvalue_9) (Math|Boolean|ANDBoolean (Variables|/Game/Tasks/DishTask/Code/PlateReplace1.PlateReplace1_C|GetIsDone? _returnvalue_10) (Variables|/Game/Tasks/DishTask/Code/PlateReplace2.PlateReplace2_C|GetIsDone? _returnvalue_11) (Variables|/Game/Tasks/DishTask/Code/PlateReplace3.PlateReplace3_C|GetIsDone? _returnvalue_12) (Variables|/Game/Tasks/DishTask/Code/PlateReplace4.PlateReplace4_C|GetIsDone? _returnvalue_13) (Variables|/Game/Tasks/DishTask/Code/PlateReplace5.PlateReplace5_C|GetIsDone? _returnvalue_14))))) (Variables|Default|GetNumTasksCompleted)) _returnvalue_4)))
    (Class|DaySequenceActor|SetTimeOfDay (+ (* (/ _returnvalue_4 (Utilities|Array|Length (Utilities|Array|MakeArray (and (Variables|/Game/Tasks/BedTask/Code/BlanketReplace.BlanketReplace_C|GetIsDone? _returnvalue_5) (Variables|/Game/Tasks/BedTask/Code/PillowReplace.PillowReplace_C|GetIsDone? _returnvalue_6)) (Variables|/Game/Tasks/FoodTask/Code/FoodTask.FoodTask_C|GetIsDone? _returnvalue_7) (Variables|/Game/Tasks/ShowerTask/Code/ShowerTask.ShowerTask_C|GetIsDone? _returnvalue_8) (Variables|/Game/Tasks/PillsTask/Code/PillsPickup.PillsPickup_C|GetIsDone? _returnvalue_9) (Math|Boolean|ANDBoolean (Variables|/Game/Tasks/DishTask/Code/PlateReplace1.PlateReplace1_C|GetIsDone? _returnvalue_10) (Variables|/Game/Tasks/DishTask/Code/PlateReplace2.PlateReplace2_C|GetIsDone? _returnvalue_11) (Variables|/Game/Tasks/DishTask/Code/PlateReplace3.PlateReplace3_C|GetIsDone? _returnvalue_12) (Variables|/Game/Tasks/DishTask/Code/PlateReplace4.PlateReplace4_C|GetIsDone? _returnvalue_13) (Variables|/Game/Tasks/DishTask/Code/PlateReplace5.PlateReplace5_C|GetIsDone? _returnvalue_14))))) (Variables|Default|GetNumTasksCompleted)) _returnvalue_4))))

(fn ConstructionScript)