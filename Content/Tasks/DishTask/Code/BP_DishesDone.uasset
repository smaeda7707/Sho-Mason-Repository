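; BP_DishesDone tracks completion of the dish task and flags the sleep task through BP_Sleep1.
; BeginPlay clears DishesDone but already sets BP_Sleep1's IsTask to true.
; Every Tick looks up the five PlateReplace actors by class through nested checks that each is done and no longer a task.
; When all five pass, it sets DishesDone and sets the sleep actor's IsTask to true again, repeating each frame.
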(event EventTick
  (params (DeltaSeconds :type Float%20%28single-precision%29))
  (bind _returnvalue (Actor|GetActorOfClass "/Game/Tasks/DishTask/Code/PlateReplace1.PlateReplace1_C"))
  (if (not (Variables|/Game/Tasks/DishTask/Code/PlateReplace1.PlateReplace1_C|GetIsTask? _returnvalue))
    (if (Variables|/Game/Tasks/DishTask/Code/PlateReplace1.PlateReplace1_C|GetIsDone? _returnvalue)
      (bind _returnvalue_2 (Actor|GetActorOfClass "/Game/Tasks/DishTask/Code/PlateReplace2.PlateReplace2_C"))
      (if (not (Variables|/Game/Tasks/DishTask/Code/PlateReplace2.PlateReplace2_C|GetIsTask? _returnvalue_2))
        (if (Variables|/Game/Tasks/DishTask/Code/PlateReplace2.PlateReplace2_C|GetIsDone? _returnvalue_2)
          (bind _returnvalue_3 (Actor|GetActorOfClass "/Game/Tasks/DishTask/Code/PlateReplace3.PlateReplace3_C"))
          (if (not (Variables|/Game/Tasks/DishTask/Code/PlateReplace3.PlateReplace3_C|GetIsTask? _returnvalue_3))
            (if (Variables|/Game/Tasks/DishTask/Code/PlateReplace3.PlateReplace3_C|GetIsDone? _returnvalue_3)
              (bind _returnvalue_4 (Actor|GetActorOfClass "/Game/Tasks/DishTask/Code/PlateReplace4.PlateReplace4_C"))
              (if (not (Variables|/Game/Tasks/DishTask/Code/PlateReplace4.PlateReplace4_C|GetIsTask? _returnvalue_4))
                (if (Variables|/Game/Tasks/DishTask/Code/PlateReplace4.PlateReplace4_C|GetIsDone? _returnvalue_4)
                  (bind _returnvalue_5 (Actor|GetActorOfClass "/Game/Tasks/DishTask/Code/PlateReplace5.PlateReplace5_C"))
                  (if (not (Variables|/Game/Tasks/DishTask/Code/PlateReplace5.PlateReplace5_C|GetIsTask? _returnvalue_5))
                    (if (Variables|/Game/Tasks/DishTask/Code/PlateReplace5.PlateReplace5_C|GetIsDone? _returnvalue_5)
                      (Variables|Default|SetDishesDone true)
                      (bind _returnvalue_6 (Actor|GetActorOfClass "/Game/Tasks/BP_Sleep1.BP_Sleep1_C"))
                      (Variables|/Game/Tasks/BP_Sleep1.BP_Sleep1_C|SetIsTask? _returnvalue_6 true))))))))))))

(event EventBeginPlay
  (Variables|Default|SetDishesDone false)
  (bind _returnvalue (Actor|GetActorOfClass "/Game/Tasks/BP_Sleep1.BP_Sleep1_C"))
  (Variables|/Game/Tasks/BP_Sleep1.BP_Sleep1_C|SetIsTask? _returnvalue true))

(fn ConstructionScript)