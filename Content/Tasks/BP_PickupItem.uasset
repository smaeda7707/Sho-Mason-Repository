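; BP_PickupItem is an item that the first-person player character can pick up and hold in the left hand.
; It polls the cached character every tick, and interacting while targeting it snaps it to HandGrip_L on EquippedItem, then applies RotationInHand to EquippedItem.
; Tick derives the held state from ItemModel's attach parent, switching collision and gravity off while held and on otherwise.
; UniversalInteract and TogglePickup are stubs.
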(event EventBeginPlay
  (Variables|Default|SetIsHolding? false)
  (CallFunction|SetVariables))

(event Collision|EventActorBeginOverlap
  (params (OtherActor :type Actor%20Object%20Reference)))

(event EventPickup
  (bind _characterref (Variables|Default|GetCharacterRef))
  (bind _equippeditem (Variables|/Game/FirstPerson/Blueprints/BP_FirstPersonCharacter.BP_FirstPersonCharacter_C|GetEquippedItem _characterref))
  (Transformation|AttachComponentToComponent _equippeditem "HandGrip_L" "SnapToTarget" "SnapToTarget" "KeepRelative" true)
  (Transformation|SetRelativeRotation _equippeditem (Variables|Default|GetRotationInHand) false false))

(event EventTick
  (params (DeltaSeconds :type Float%20%28single-precision%29))
  (bind _itemmodel (Variables|Default|GetItemModel))
  (CallFunction|InteractCheck)
  (bind _output_get (Variables|Default|SetIsHolding? (== (Variables|/Game/FirstPerson/Blueprints/BP_FirstPersonCharacter.BP_FirstPersonCharacter_C|GetEquippedItem (Variables|Default|GetCharacterRef)) (Transformation|GetAttachParent _itemmodel))))
  (if _output_get
    (Collision|SetCollisionEnabled _itemmodel "NoCollision")
    (Physics|SetEnableGravity _itemmodel false)
    (else
      (Collision|SetCollisionEnabled _itemmodel "QueryAndPhysics")
      (Physics|SetEnableGravity _itemmodel true))))

(fn ConstructionScript)

(fn InteractCheck
  (bind _characterref (Variables|Default|GetCharacterRef))
  (if (Variables|Default|GetEndTick)
    (if (and (Variables|/Game/FirstPerson/Blueprints/BP_FirstPersonCharacter.BP_FirstPersonCharacter_C|GetIsInteracting? _characterref) (== (Variables|/Game/FirstPerson/Blueprints/BP_FirstPersonCharacter.BP_FirstPersonCharacter_C|GetHit%20Actor _characterref) self))
      (CallFunction|Pickup))))

(fn TogglePickup)

(fn SetVariables
  (Variables|Default|SetEndTick true)
  (bind _asbp_first_person_character (Utilities|Casting|CastToBP_FirstPersonCharacter (Game|GetPlayerCharacter 0)))
  (Variables|Default|SetCharacterRef _asbp_first_person_character))

(fn UniversalInteract
  (params (Interactor :type Character%20Object%20Reference))
  (return false))