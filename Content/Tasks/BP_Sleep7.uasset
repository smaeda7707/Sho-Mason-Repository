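; BP_Sleep7 is a sleep task actor whose invisible mattress plays a cutscene, then sends the game to the main menu.
; Tick polls until IsTask is set, enables mattress collision, and fires once when the interacting player's HitActor is this actor.
; It disables input for the sequence's duration, then opens MainMenuMap, pauses, and switches to cursor and UI-only input.
; UniversalInteract is a stub returning false, so interaction relies entirely on Tick.
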(event EventBeginPlay
  (bind _mattress (Variables|Default|Getmattress))
  (Rendering|SetVisibility _mattress false false)
  (Collision|SetCollisionEnabled _mattress "NoCollision")
  (Variables|Default|SetIsUsing? false)
  (Variables|Default|SetIsDone? false)
  (Variables|Default|SetEndTick true)
  (Variables|Default|SetIsTask? false)
  (bind _asbp_first_person_character (Utilities|Casting|CastToBP_FirstPersonCharacter (Game|GetPlayerCharacter 0)))
  (Variables|Default|SetCharacterRef _asbp_first_person_character))

(event EventTick
  (params (DeltaSeconds :type Float%20%28single-precision%29))
  (bind _returnvalue (Game|GetPlayerCharacter 0))
  (bind _characterref (Variables|Default|GetCharacterRef))
  (bind _sequencereference (Variables|Default|GetSequenceReference))
  (bind _sequenceplayer (Variables|/Script/LevelSequence.LevelSequenceActor|GetSequencePlayer _sequencereference))
  (if (Variables|Default|GetEndTick)
    (if (Variables|Default|GetIsTask?)
      (Collision|SetCollisionEnabled (Variables|Default|Getmattress) "QueryAndProbe")
      (if (and (Variables|/Game/FirstPerson/Blueprints/BP_FirstPersonCharacter.BP_FirstPersonCharacter_C|GetIsInteracting? _characterref) (== (Variables|/Game/FirstPerson/Blueprints/BP_FirstPersonCharacter.BP_FirstPersonCharacter_C|GetHit%20Actor _characterref) self))
        (Variables|Default|SetIsUsing? true)
        (Variables|Default|SetEndTick false)
        (Sequencer|Player|Play _sequenceplayer :!class /Script/MovieScene.MovieSceneSequencePlayer)
        (Input|DisableInput _returnvalue 0)
        (Utilities|FlowControl|Delay (Class|TimeManagementBlueprintLibrary|ToSeconds(QualifiedFrameTime) (Media|MediaPlayer|GetDuration _sequenceplayer)))
        (Input|EnableInput _returnvalue 0)
        (Variables|Default|SetIsUsing? false)
        (Game|OpenLevel(byObjectReference) "/Game/Alexs_Stuff/MainMenuMap.MainMenuMap")
        (Game|SetGamePaused true)
        (Variables|/Script/Engine.PlayerController|SetbShowMouseCursor (Game|GetPlayerController 0) true)
        (Input|SetInputModeUIOnly 0 0 "DoNotLock" false)))))

(fn ConstructionScript)

(fn UniversalInteract
  (params (Interactor :type Character%20Object%20Reference))
  (return false))