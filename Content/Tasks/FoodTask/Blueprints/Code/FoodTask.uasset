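; FoodTask is an interactable food task actor that the player completes by eating it.
; BeginPlay caches the first-person character, and Tick polls whether that character is interacting with this actor as its hit target.
; On a match, ToggleEat marks the task done, clears its task flag and destroys the actor.
; The UniversalInteract function is a stub that returns false, so interaction relies on polling.
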(event Custom|Toggle%20Eat
  (Variables|Default|SetEndTick false)
  (Variables|Default|SetIsTask? false)
  (Variables|Default|SetIsDone? true)
  (Actor|DestroyActor))

(event EventBeginPlay
  (Variables|Default|SetEndTick true)
  (Variables|Default|SetIsDone? false)
  (Variables|Default|SetIsTask? true)
  (bind _asbp_first_person_character (Utilities|Casting|CastToBP_FirstPersonCharacter (Game|GetPlayerCharacter 0)))
  (Variables|Default|SetCharacterRef _asbp_first_person_character))

(event EventTick
  (params (DeltaSeconds :type Float%20%28single-precision%29))
  (bind _characterref (Variables|Default|GetCharacterRef))
  (if (Variables|Default|GetEndTick)
    (if (and (Variables|/Game/FirstPerson/Blueprints/BP_FirstPersonCharacter.BP_FirstPersonCharacter_C|GetIsInteracting? _characterref) (== (Variables|/Game/FirstPerson/Blueprints/BP_FirstPersonCharacter.BP_FirstPersonCharacter_C|GetHit%20Actor _characterref) self))
      (if (Variables|Default|GetIsTask?)
        (CallFunction|ToggleEat)))))

(fn ConstructionScript)

(fn UniversalInteract
  (params (Interactor :type Character%20Object%20Reference))
  (return false))