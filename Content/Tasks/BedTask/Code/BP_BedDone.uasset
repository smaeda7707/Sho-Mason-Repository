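; BP_BedDone tracks completion of the bed task and unlocks the pills pickup task that follows it.
; Every Tick until done, it looks up the PillowReplace and BlanketReplace actors by class and checks that each has IsTask cleared and IsDone set.
; When both pass, it latches BedDone and sets IsTask on the PillsPickup actor.
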(event EventBeginPlay
  (Variables|Default|SetBedDone false))

(event EventTick
  (params (DeltaSeconds :type Float%20%28single-precision%29))
  (if (not (Variables|Default|GetBedDone))
    (bind _returnvalue (Actor|GetActorOfClass "/Game/Tasks/BedTask/Code/PillowReplace.PillowReplace_C"))
    (if (not (Variables|/Game/Tasks/BedTask/Code/PillowReplace.PillowReplace_C|GetIsTask? _returnvalue))
      (if (Variables|/Game/Tasks/BedTask/Code/PillowReplace.PillowReplace_C|GetIsDone? _returnvalue)
        (bind _returnvalue_2 (Actor|GetActorOfClass "/Game/Tasks/BedTask/Code/BlanketReplace.BlanketReplace_C"))
        (if (not (Variables|/Game/Tasks/BedTask/Code/BlanketReplace.BlanketReplace_C|GetIsTask? _returnvalue_2))
          (if (Variables|/Game/Tasks/BedTask/Code/BlanketReplace.BlanketReplace_C|GetIsDone? _returnvalue_2)
            (Variables|Default|SetBedDone true)
            (bind _returnvalue_3 (Actor|GetActorOfClass "/Game/Tasks/PillsTask/Code/PillsPickup.PillsPickup_C"))
            (Variables|/Game/Tasks/PillsTask/Code/PillsPickup.PillsPickup_C|SetIsTask? _returnvalue_3 true)))))))

(fn ConstructionScript)