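; BP_Generator is a generator for the electricity task that the player switches off and on.
; Tick polls the first-person character's IsInteracting and HitActor, then toggles IsOn after a short Delay.
; It starts on, and the first switch back on sets IsDone and clears IsTask, completing the task once.
; UniversalInteract only returns false, so interaction relies entirely on that polling.
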(event EventBeginPlay
  (Variables|Default|SetIsDone? false)
  (Variables|Default|SetIsTask? true)
  (Variables|Default|SetIsOn? true)
  (bind _asbp_first_person_character (Utilities|Casting|CastToBP_FirstPersonCharacter (Game|GetPlayerCharacter 0)))
  (Variables|Default|SetCharacterRef _asbp_first_person_character))

(event EventTick
  (params (DeltaSeconds :type Float%20%28single-precision%29))
  (bind _characterref (Variables|Default|GetCharacterRef))
  (if (and (Variables|/Game/FirstPerson/Blueprints/BP_FirstPersonCharacter.BP_FirstPersonCharacter_C|GetIsInteracting? _characterref) (== (Variables|/Game/FirstPerson/Blueprints/BP_FirstPersonCharacter.BP_FirstPersonCharacter_C|GetHit%20Actor _characterref) self))
    (Utilities|FlowControl|Delay 0.2)
    (if (Variables|Default|GetIsOn?)
      (Variables|Default|SetIsOn? false)
      (else
        (Variables|Default|SetIsOn? true)
        (if (Variables|Default|GetIsTask?)
          (Variables|Default|SetIsDone? true)
          (Variables|Default|SetIsTask? false))))))

(fn ConstructionScript)

(fn UniversalInteract
  (params (Interactor :type Character%20Object%20Reference))
  (return false))