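; Back door actor for the lock-door task, which the player can open, close, lock and unlock.
; Each Tick it polls the first-person character for an interaction targeting it, closing if open, toggling the lock if the house key is held, or opening if unlocked.
; The first lock marks the task done.
; Open and close calls first set the door timeline's play rate from their respective durations.
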(event EventBeginPlay
  (Variables|Default|SetLockDoorTaskDone false)
  (Variables|Default|SetLockDoorTask true)
  (Variables|Default|SetIsLocked? false)
  (Variables|Default|SetIsOpen? false)
  (bind _asbp_first_person_character (Utilities|Casting|CastToBP_FirstPersonCharacter (Game|GetPlayerCharacter 0)))
  (Variables|Default|SetCharacterRef _asbp_first_person_character))

(event EventTick
  (params (DeltaSeconds :type Float%20%28single-precision%29))
  (bind _open_door_time (Variables|Default|GetOpen%20Door%20Time))
  (bind _characterref (Variables|Default|GetCharacterRef))
  (if (and (Variables|/Game/FirstPerson/Blueprints/BP_FirstPersonCharacter.BP_FirstPersonCharacter_C|GetIsInteracting? _characterref) (== (Variables|/Game/FirstPerson/Blueprints/BP_FirstPersonCharacter.BP_FirstPersonCharacter_C|GetHit%20Actor _characterref) self))
    (if (Variables|Default|GetIsOpen?)
      (Components|Timeline|SetPlayRate _open_door_time (/ 1.0 (Variables|Default|GetCloseTime)))
      (CallFunction|CloseDoor)
      (else
        (bind _returnvalue (Actor|GetActorOfClass "/Game/Tasks/LockBackDoorTask/Code/BP_HouseKey.BP_HouseKey_C"))
        (if (Variables|/Game/Tasks/BP_PickupItem.BP_PickupItem_C|GetIsHolding? _returnvalue)
          (if (Variables|Default|GetIsLocked?)
            (Variables|Default|SetIsLocked? false)
            (else
              (Variables|Default|SetIsLocked? true)
              (if (Variables|Default|GetLockDoorTask)
                (Variables|Default|SetLockDoorTask false)
                (Variables|Default|SetLockDoorTaskDone true))))
          (elif (not (Variables|Default|GetIsLocked?))
            (Components|Timeline|SetPlayRate _open_door_time (/ 1.0 (Variables|Default|GetOpenTime)))
            (CallFunction|OpenDoor)))))))

(fn ConstructionScript
  (|CallParentFunction))