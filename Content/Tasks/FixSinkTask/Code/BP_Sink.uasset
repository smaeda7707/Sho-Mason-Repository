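; BP_Sink is the sink in a fix-sink task, repaired by the player with a held BP_Wrench.
; While IsTask is set, Tick polls for the player interacting with this actor and wrench in hand, then calls FixSink.
; FixSink stops the check, marks the task done, counts fixes and spawns a water effect at a hardcoded location, or an inactive one on the second fix.
; UniversalInteract is a stub returning false.
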(event Custom|FixSink
  (Variables|Default|SetEndTick false)
  (Variables|Default|SetIsTask? false)
  (Variables|Default|SetIsDone? true)
  (bind _output_get (Variables|Default|SetTimesFixed (+ (Variables|Default|GetTimesFixed) 1)))
  (if (== _output_get 2)
    (Niagara|SpawnSystematLocation "/Game/Tasks/DishTask/Code/SinkWaterSystem.SinkWaterSystem" "0, 0, 0" "0, 0, 0" "1.000000,1.000000,1.000000" true false)
    (else
      (Niagara|SpawnSystematLocation "/Game/Tasks/DishTask/Code/SinkWaterSystem.SinkWaterSystem" "-938.000000,144.000000,280.000000" "0, 0, 0" "0.100000,0.100000,0.100000" false))))

(event EventBeginPlay
  (Variables|Default|SetTimesFixed 0)
  (Variables|Default|SetIsTask? false)
  (Variables|Default|SetEndTick true)
  (Variables|Default|SetIsDone? false)
  (bind _asbp_first_person_character (Utilities|Casting|CastToBP_FirstPersonCharacter (Game|GetPlayerCharacter 0)))
  (Variables|Default|SetCharacterRef _asbp_first_person_character))

(event EventTick
  (params (DeltaSeconds :type Float%20%28single-precision%29))
  (bind _characterref (Variables|Default|GetCharacterRef))
  (if (Variables|Default|GetEndTick)
    (if (Variables|Default|GetIsTask?)
      (if (and (Variables|/Game/FirstPerson/Blueprints/BP_FirstPersonCharacter.BP_FirstPersonCharacter_C|GetIsInteracting? _characterref) (== (Variables|/Game/FirstPerson/Blueprints/BP_FirstPersonCharacter.BP_FirstPersonCharacter_C|GetHit%20Actor _characterref) self))
        (bind _returnvalue (Actor|GetActorOfClass "/Game/Tasks/FixSinkTask/Code/BP_Wrench.BP_Wrench_C"))
        (if (Variables|/Game/Tasks/BP_PickupItem.BP_PickupItem_C|GetIsHolding? _returnvalue)
          (CallFunction|FixSink))))))

(fn ConstructionScript)

(fn UniversalInteract
  (params (Interactor :type Character%20Object%20Reference))
  (return false))